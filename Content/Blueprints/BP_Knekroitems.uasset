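; BP_Knekroitems is an interactable pickup item that the first-person character can carry in hand.
; The construction script sets its mesh and material from the ItemSelected choice, covering five themed props such as a Pokeball, bat and hat.
; Box overlaps toggle a widget's visibility.
; Interact finds an overlapping character, hides the widget, deactivates the box and attaches to the character's ItemHand component.
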(event OnComponentBeginOverlap(Box)
  (params (OverlappedComponent :type Primitive%20Component%20Object%20Reference) (OtherActor :type Actor%20Object%20Reference) (OtherComp :type Primitive%20Component%20Object%20Reference) (OtherBodyIndex :type Integer) (bFromSweep :type Boolean) (SweepResult :type Hit%20Result%20Structure%20%28by%20ref%29))
  (Rendering|SetVisibility (Variables|Default|GetWidget) true false))

(event OnComponentEndOverlap(Box)
  (params (OverlappedComponent :type Primitive%20Component%20Object%20Reference) (OtherActor :type Actor%20Object%20Reference) (OtherComp :type Primitive%20Component%20Object%20Reference) (OtherBodyIndex :type Integer))
  (Rendering|SetVisibility (Variables|Default|GetWidget) false false))

(event EventInteract
  (bind _array_element (Utilities|Array|ForEachLoopwithBreak (Collision|GetOverlappingActors (Variables|Default|GetBox) "/Game/FirstPerson/Blueprints/BP_FirstPersonCharacter.BP_FirstPersonCharacter_C" :!class /Script/Engine.PrimitiveComponent) :!label _label)
    (:LoopBody
      (bind _asbp_first_person_character (Utilities|Casting|CastToBP_FirstPersonCharacter _array_element))
      (Rendering|SetVisibility (Variables|Default|GetWidget) false false)
      (Components|Activation|SetActive (Variables|Default|GetBox) false false)
      (Transformation|AttachComponentToComponent (Variables|/Game/FirstPerson/Blueprints/BP_FirstPersonCharacter.BP_FirstPersonCharacter_C|GetItemHand _asbp_first_person_character) "" "SnapToTarget" "KeepRelative" "KeepRelative" true)
      (goto _label Break))))

(fn ConstructionScript
  (bind _staticmesh (Variables|Default|GetStaticMesh))
  (bind _staticmesh_2 (Variables|Default|GetStaticMesh))
  (switch Utilities|FlowControl|Switch|SwitchonEnum_Items (Variables|Default|Getitem_selected)
    (:NewEnumerator0
      (Components|StaticMesh|SetStaticMesh _staticmesh "/Game/IlloJam/Imports/thpsct/Pokeball.Pokeball")
      (Rendering|Material|SetMaterial _staticmesh_2 0 "/Game/IlloJam/Imports/thpsct/SetupGayming/Material_009.Material_009"))
    (:NewEnumerator1
      (Components|StaticMesh|SetStaticMesh _staticmesh "/Game/IlloJam/Imports/BateBaseball.BateBaseball")
      (Rendering|Material|SetMaterial _staticmesh_2 0 "/Game/Models/Wood.Wood"))
    (:NewEnumerator2
      (Components|StaticMesh|SetStaticMesh _staticmesh "/Game/IlloJam/Imports/thpsct/ruedita.ruedita")
      (Rendering|Material|SetMaterial _staticmesh_2 0 "/Game/IlloJam/Imports/thpsct/SetupGayming/Material_009.Material_009"))
    (:NewEnumerator3
      (Components|StaticMesh|SetStaticMesh _staticmesh "/Game/IlloJam/Imports/thpsct/AirHorn.AirHorn")
      (Rendering|Material|SetMaterial _staticmesh_2 0 0))
    (:NewEnumerator4
      (Components|StaticMesh|SetStaticMesh _staticmesh "/Game/IlloJam/Imports/thpsct/source/Mario_Hat.Mario_Hat")
      (Rendering|Material|SetMaterial _staticmesh_2 0 "/Game/IlloJam/Imports/thpsct/source/03_-_Default.03_-_Default"))))