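; BP_KeyKnekro is an interactable pickup item that the first-person character can take in hand.
; The construction script sets its static mesh from the ItemSelected enum, one mesh per item type.
; Overlapping the Box shows a prompt widget and leaving hides it.
; Interact finds an overlapping BP_FirstPersonCharacter, hides the widget, deactivates the Box and attaches the item to that character's ItemHand.
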(event OnComponentBeginOverlap(Box)
  (params (OverlappedComponent :type Primitive%20Component%20Object%20Reference) (OtherActor :type Actor%20Object%20Reference) (OtherComp :type Primitive%20Component%20Object%20Reference) (OtherBodyIndex :type Integer) (bFromSweep :type Boolean) (SweepResult :type Hit%20Result%20Structure%20%28by%20ref%29))
  (Rendering|SetVisibility (Variables|Default|GetWidget) true false))

(event OnComponentEndOverlap(Box)
  (params (OverlappedComponent :type Primitive%20Component%20Object%20Reference) (OtherActor :type Actor%20Object%20Reference) (OtherComp :type Primitive%20Component%20Object%20Reference) (OtherBodyIndex :type Integer))
  (Rendering|SetVisibility (Variables|Default|GetWidget) false false))

(event EventBeginPlay)

(event EventInteract
  (bind _array_element (Utilities|Array|ForEachLoopwithBreak (Collision|GetOverlappingActors (Variables|Default|GetBox) "/Game/FirstPerson/Blueprints/BP_FirstPersonCharacter.BP_FirstPersonCharacter_C" :!class /Script/Engine.PrimitiveComponent) :!label _label)
    (:LoopBody
      (bind _asbp_first_person_character (Utilities|Casting|CastToBP_FirstPersonCharacter _array_element))
      (Rendering|SetVisibility (Variables|Default|GetWidget) false false)
      (Components|Activation|SetActive (Variables|Default|GetBox) false false)
      (Transformation|AttachComponentToComponent (Variables|/Game/FirstPerson/Blueprints/BP_FirstPersonCharacter.BP_FirstPersonCharacter_C|GetItemHand _asbp_first_person_character) "" "SnapToTarget" "KeepRelative" "KeepRelative" true)
      (goto _label Break))))

(event EventTick
  (params (DeltaSeconds :type Float%20%28single-precision%29)))

(fn ConstructionScript
  (bind _staticmesh (Variables|Default|GetStaticMesh))
  (switch Utilities|FlowControl|Switch|SwitchonEnum_Items (Variables|Default|Getitem_selected)
    (:NewEnumerator0
      (Components|StaticMesh|SetStaticMesh _staticmesh "/Game/StarterContent/Shapes/Shape_Trim.Shape_Trim"))
    (:NewEnumerator1
      (Components|StaticMesh|SetStaticMesh _staticmesh "/Game/IlloJam/Imports/BateBaseball.BateBaseball"))
    (:NewEnumerator2
      (Components|StaticMesh|SetStaticMesh _staticmesh "/Game/Models/kart_Neumaticos.kart_Neumaticos"))
    (:NewEnumerator3
      (Components|StaticMesh|SetStaticMesh _staticmesh "/Game/Models/Stadium/NascarStadium_polySurface75.NascarStadium_polySurface75"))
    (:NewEnumerator4
      (Components|StaticMesh|SetStaticMesh _staticmesh "/Game/Models/Character/Clothes/dress.dress"))))