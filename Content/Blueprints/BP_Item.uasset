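; Pickup item whose ItemSelected type sets its mesh in the Construction Script, with most types tied to a minigame.
; On BeginPlay it destroys itself if the matching O_GameInstance flag is set; the Knife has no such check.
; Box overlap toggles a widget, and Interact attaches the item to the overlapping character's hand_r socket.
; The Knife cannot be picked up and only plays a "Notyet2" sound.
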(event OnComponentBeginOverlap(Box)
  (params (OverlappedComponent :type Primitive%20Component%20Object%20Reference) (OtherActor :type Actor%20Object%20Reference) (OtherComp :type Primitive%20Component%20Object%20Reference) (OtherBodyIndex :type Integer) (bFromSweep :type Boolean) (SweepResult :type Hit%20Result%20Structure%20%28by%20ref%29))
  (Rendering|SetVisibility (Variables|Default|GetWidget) true false))

(event OnComponentEndOverlap(Box)
  (params (OverlappedComponent :type Primitive%20Component%20Object%20Reference) (OtherActor :type Actor%20Object%20Reference) (OtherComp :type Primitive%20Component%20Object%20Reference) (OtherBodyIndex :type Integer))
  (Rendering|SetVisibility (Variables|Default|GetWidget) false false))

(event EventBeginPlay
  (bind _aso_game_instance (Utilities|Casting|CastToO_GameInstance (Game|GetGameInstance)))
  (Utilities|FlowControl|Sequence
    (:then_0
      (if (and (Variables|/Game/IlloJam/Blueprints/O_GameInstance.O_GameInstance_C|GetBackrooms _aso_game_instance) (Utilities|Enum|Equal(Enum) (Variables|Default|Getitem_selected) "NewEnumerator0"))
        (Actor|DestroyActor :!label _label)))
    (:then_1
      (if (and (Variables|/Game/IlloJam/Blueprints/O_GameInstance.O_GameInstance_C|GetBaseball _aso_game_instance) (Utilities|Enum|Equal(Enum) (Variables|Default|Getitem_selected) "NewEnumerator1"))
        (goto _label)))
    (:then_2
      (if (and (Variables|/Game/IlloJam/Blueprints/O_GameInstance.O_GameInstance_C|GetFrogger _aso_game_instance) (Utilities|Enum|Equal(Enum) (Variables|Default|Getitem_selected) "NewEnumerator3"))
        (goto _label)))
    (:then_3
      (if (and (Variables|/Game/IlloJam/Blueprints/O_GameInstance.O_GameInstance_C|GetKarts _aso_game_instance) (Utilities|Enum|Equal(Enum) (Variables|Default|Getitem_selected) "NewEnumerator2"))
        (goto _label)))
    (:then_4
      (if (and (Variables|/Game/IlloJam/Blueprints/O_GameInstance.O_GameInstance_C|GetPlatformer _aso_game_instance) (Utilities|Enum|Equal(Enum) (Variables|Default|Getitem_selected) "NewEnumerator4"))
        (goto _label)))))

(event EventInteract
  (if (Utilities|Enum|Equal(Enum) (Variables|Default|Getitem_selected) "NewEnumerator5")
    (Audio|PlaySound2D "/Game/IlloJam/Audio/notyet2.notyet2" 1.0 1.0 0.0 0 0)
    (else
      (bind _array_element (Utilities|Array|ForEachLoopwithBreak (Collision|GetOverlappingActors (Variables|Default|GetBox) "/Game/ThirdPerson/Blueprints/BP_CustomThirdPersonCharacter.BP_CustomThirdPersonCharacter_C" :!class /Script/Engine.PrimitiveComponent) :!label _label)
        (:LoopBody
          (bind _asbp_custom_third_person_character (Utilities|Casting|CastToBP_CustomThirdPersonCharacter _array_element))
          (Rendering|SetVisibility (Variables|Default|GetWidget) false false)
          (Components|Activation|SetActive (Variables|Default|GetBox) false false)
          (Transformation|AttachComponentToComponent (Variables|/Script/Engine.Character|GetMesh _asbp_custom_third_person_character) "hand_r" "SnapToTarget" "KeepRelative" "KeepRelative" true)
          (goto _label Break))))))

(fn ConstructionScript
  (bind _staticmesh (Variables|Default|GetStaticMesh))
  (switch Utilities|FlowControl|Switch|SwitchonEnum_Items (Variables|Default|Getitem_selected)
    (:NewEnumerator0
      (Components|StaticMesh|SetStaticMesh _staticmesh "/Game/IlloJam/Imports/thpsct/Pokeball.Pokeball"))
    (:NewEnumerator1
      (Components|StaticMesh|SetStaticMesh _staticmesh "/Game/IlloJam/Imports/BateBaseball.BateBaseball"))
    (:NewEnumerator2
      (Components|StaticMesh|SetStaticMesh _staticmesh "/Game/IlloJam/Imports/thpsct/ruedita.ruedita"))
    (:NewEnumerator3
      (Components|StaticMesh|SetStaticMesh _staticmesh "/Game/IlloJam/Imports/thpsct/AirHorn.AirHorn"))
    (:NewEnumerator4
      (Components|StaticMesh|SetStaticMesh _staticmesh "/Game/IlloJam/Imports/thpsct/source/Mario_Hat.Mario_Hat"))
    (:NewEnumerator5
      (Components|StaticMesh|SetStaticMesh _staticmesh "/Game/IlloJam/Imports/thpsct/fkni.fkni"))))