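; BP_KnekroAI is the AI-driven Knekro pawn that chases the player while playing random sounds.
; Tick issues AIMoveTo toward the first player's character every frame.
; Tick also feeds a two-second Delay into the Audioloco event, which plays a random entry from RandomSound, so sounds repeat periodically.
; The BT_Knekro behavior tree launch is disconnected and never runs, leaving movement entirely to Tick.
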(event Custom|Audio%20loco
  (Default|PlayAudio (.OutItem (Utilities|Array|Random (Variables|Default|GetRandomSound)))))

(event EventTick
  (params (DeltaSeconds :type Float%20%28single-precision%29))
  (bind _returnvalue (Game|GetPlayerCharacter 0))
  (Utilities|FlowControl|Sequence
    (:then_0
      (Utilities|FlowControl|Delay 2.0)
      (CallFunction|AudioLoco))
    (:then_1
      (AI|AIMoveTo self (Transformation|GetActorLocation _returnvalue) _returnvalue 5.0 false))))

(event EventPossessed
  (params (NewController :type Controller%20Object%20Reference)))

(fn ConstructionScript)