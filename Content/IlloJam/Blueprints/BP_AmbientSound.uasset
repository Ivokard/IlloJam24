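; BP_AmbientSound plays a configurable sound as non-spatial 2D audio, optionally starting on BeginPlay.
; PlayAudio calls PlaySound2D with the set volume and pitch, then waits for the sound's duration.
; When Loop is enabled it calls itself again, so looping is driven by the delay rather than by the sound asset, and the wait ignores the pitch multiplier.
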(event Custom|PlayAudio
  (Audio|PlaySound2D (Variables|Default|GetSound) (Variables|Default|GetVolume) (Variables|Default|GetPitch) 0.0 0 0)
  (Utilities|FlowControl|Delay (Variables|/Script/Engine.SoundBase|GetDuration (Variables|Default|GetSound)))
  (if (Variables|Default|GetLoop)
    (CallFunction|PlayAudio)))

(event EventBeginPlay
  (if (Variables|Default|GetPlayAtStart)
    (CallFunction|PlayAudio)))

(fn ConstructionScript)