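; BP_CheckpointSystem tracks actors' checkpoint progress and counts laps, with add and remove functions maintaining the checkpoint total.
; TrackActor advances an actor's BP_CheckpointData record on the next sequential ID, or any ID after the last, adding a lap when wrapping to zero.
; NewTracked creates records for an empty list, but also for every non-matching entry during the loop, so duplicates can accumulate.
; Debug prints trace the checks.
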(event EventBeginPlay)

(event Collision|EventActorBeginOverlap
  (params (OtherActor :type Actor%20Object%20Reference)))

(event EventTick
  (params (DeltaSeconds :type Float%20%28single-precision%29)))

(fn ConstructionScript)

(fn TrackActor
  (params (Actor :type Object%20Object%20Reference) (CheckpointId :type Integer))
  (bind _tracked (Variables|Default|GetTracked))
  (LocalVariables|SetCurrentCheckpointId CheckpointId)
  (if (== (Utilities|Array|Length _tracked) 0)
    (bind _asactor (Utilities|Casting|CastToActor Actor))
    (CallFunction|NewTracked _asactor (LocalVariables|GetCurrentCheckpointId))
    (else
      (for _array_element _tracked
        (Development|PrintText (Utilities|Text|FormatText "SCI: {sci} | CID: {cid}" (LocalVariables|GetCurrentCheckpointId) (+ (Variables|/Game/IlloJam/Blueprints/BP_CheckpointData.BP_CheckpointData_C|GetCheckpointId _array_element) 1)))
        (if (== (Variables|/Game/IlloJam/Blueprints/BP_CheckpointData.BP_CheckpointData_C|GetActor _array_element) Actor)
          (if (or (== (+ (Variables|/Game/IlloJam/Blueprints/BP_CheckpointData.BP_CheckpointData_C|GetCheckpointId _array_element) 1) (LocalVariables|GetCurrentCheckpointId)) (>= (+ (Variables|/Game/IlloJam/Blueprints/BP_CheckpointData.BP_CheckpointData_C|GetCheckpointId _array_element) 1) (Variables|Default|GetCheckpointCount)))
            (bind _output_get (Variables|/Game/IlloJam/Blueprints/BP_CheckpointData.BP_CheckpointData_C|SetLastCheckpointId _array_element (Variables|/Game/IlloJam/Blueprints/BP_CheckpointData.BP_CheckpointData_C|GetCheckpointId _array_element)))
            (bind _output_get_2 (Variables|/Game/IlloJam/Blueprints/BP_CheckpointData.BP_CheckpointData_C|SetCheckpointId _array_element (LocalVariables|GetCurrentCheckpointId)))
            (Development|PrintString (Utilities|String|ToString(Integer) _output_get))
            (if (and (== _output_get_2 0) (== (Variables|/Game/IlloJam/Blueprints/BP_CheckpointData.BP_CheckpointData_C|GetLastCheckpointId _array_element) (- (Variables|Default|GetCheckpointCount) 1)))
              (Development|PrintString "LAP")
              (Variables|/Game/IlloJam/Blueprints/BP_CheckpointData.BP_CheckpointData_C|SetLap _array_element (+ (Variables|/Game/IlloJam/Blueprints/BP_CheckpointData.BP_CheckpointData_C|GetLap _array_element) 1))))
          (else
            (bind _asactor_2 (Utilities|Casting|CastToActor Actor))
            (CallFunction|NewTracked _asactor_2 (LocalVariables|GetCurrentCheckpointId))))))))

(fn NewTracked
  (params (Actor :type Actor%20Object%20Reference) (CheckpointId :type Integer))
  (Development|PrintString "UNTRACKED")
  (bind _returnvalue (Game|ConstructObjectfromClass "/Game/IlloJam/Blueprints/BP_CheckpointData.BP_CheckpointData_C"))
  (bind _data (Default|Instantiate _returnvalue Actor CheckpointId))
  (Utilities|Array|Add (Variables|Default|GetTracked) _data))

(fn AddCheckpoint
  (Math|Integer|IncrementInt (Variables|Default|GetCheckpointCount)))

(fn RemoveCheckpoint
  (Math|Integer|DecrementInt (Variables|Default|GetCheckpointCount)))