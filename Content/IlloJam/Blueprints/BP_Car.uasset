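; BP_Car is a moving car obstacle for a Frogger-style game that resets BP_JuanFrogger on overlap.
; On BeginPlay it varies its Speed by up to ten percent either way and destroys itself after a fixed lifetime.
; Tick teleports it along world Y by Speed, without sweep.
; A Delay on Tick also fires CallNextCar repeatedly, spaced by NextCarDelay.
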(event EventTick
  (params (DeltaSeconds :type Float%20%28single-precision%29))
  (bind _defaultsceneroot (Variables|Default|GetDefaultSceneRoot))
  (bind _returnvalue (Transformation|GetWorldLocation _defaultsceneroot))
  (bind (_x _y _z) (Math|Vector|BreakVector _returnvalue))
  (Transformation|SetWorldLocation (Variables|Default|GetDefaultSceneRoot) (Math|Vector|MakeVector _x (+ (* DeltaSeconds (Variables|Default|GetSpeed)) _y) _z) false true)
  (Utilities|FlowControl|Delay (Variables|Default|GetNextCarDelay))
  (Default|CallNextCar))

(event EventBeginPlay
  (Variables|Default|SetSpeed (+ (Variables|Default|GetSpeed) (Math|Random|RandomFloatinRange (* (/ (Variables|Default|GetSpeed) 1e+01) -1.0) (/ (Variables|Default|GetSpeed) 1e+01))))
  (Utilities|FlowControl|Delay 15.0)
  (Actor|DestroyActor))

(event Collision|EventActorBeginOverlap
  (params (OtherActor :type Actor%20Object%20Reference))
  (bind _asbp_juan_frogger (Utilities|Casting|CastToBP_JuanFrogger OtherActor))
  (Default|Reset _asbp_juan_frogger))

(fn ConstructionScript)