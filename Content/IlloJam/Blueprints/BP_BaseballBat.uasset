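; BP_BaseballBat is a baseball bat that follows the mouse and tracks whether it is in a hitting swing.
; Each tick it normalizes the cursor's viewport X, accounting for viewport scale, and maps it to the yaw of its Pivot.
; Cursor movement refreshes a countdown set by HitTime.
; Hits is true only while that timer runs, the cursor is within a central horizontal band, and it is moving leftward.
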(event EventTick
  (params (DeltaSeconds :type Float%20%28single-precision%29))
  (bind _output_get (Variables|Default|SetTimeSinceMoved (- (Variables|Default|GetTimeSinceMoved) DeltaSeconds)))
  (Utilities|FlowControl|Sequence
    (:then_0
      (bind _returnvalue (Class|WidgetLayoutLibrary|GetMousePositiononViewport))
      (Variables|Default|SetLastXPos (Variables|Default|GetCurrentXPos))
      (Variables|Default|SetCurrentXPos (/ (* (.X (Math|Vector2D|BreakVector2D _returnvalue)) (Class|WidgetLayoutLibrary|GetViewportScale)) (.X (Math|Vector2D|BreakVector2D (Viewport|GetViewportSize)))))
      (Transformation|SetRelativeRotation (Variables|Default|GetPivot) (Math|Rotator|MakeRotator 0.0 0.0 (* (- (/ (* (.X (Math|Vector2D|BreakVector2D _returnvalue)) (Class|WidgetLayoutLibrary|GetViewportScale)) (.X (Math|Vector2D|BreakVector2D (Viewport|GetViewportSize)))) 0.5) 175.0)) false false)
      (if (!= (Variables|Default|GetCurrentXPos) (Variables|Default|GetLastXPos))
        (Variables|Default|SetTimeSinceMoved (Variables|Default|GetHitTime))))
    (:then_1
      (bind _output_get_2 (Variables|Default|SetHits (Math|Boolean|ANDBoolean (> _output_get 0.0) (and (>= (Variables|Default|GetCurrentXPos) 0.15) (<= (Variables|Default|GetCurrentXPos) 0.8)) (> (Variables|Default|GetLastXPos) (Variables|Default|GetCurrentXPos))))))))

(event Input|MouseEvents|MouseX
  (params (AxisValue :type Float%20%28single-precision%29))
  (Development|PrintString "Hello"))

(fn ConstructionScript)