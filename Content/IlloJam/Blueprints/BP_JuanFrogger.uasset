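; BP_JuanFrogger is a Frogger-style player that hops one grid square at a time within min and max limits.
; While Active, each movement axis steps X or Y once per press, re-arming at zero input, and plays Boing.
; Tick applies those coordinates to the root at zero height.
; Reset teleports back to the position saved at BeginPlay and calls the Reseted dispatcher.
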(event Custom|Reset
  (bind _resetpos (Variables|Default|GetResetPos))
  (bind (_x _y) (Math|Vector|BreakVector _resetpos))
  (Transformation|SetWorldLocation (Variables|Default|GetDefaultSceneRoot) _resetpos false true)
  (Variables|Default|SetX (Math|Float|Truncate _x))
  (Variables|Default|SetY (Math|Float|Truncate _y))
  (Default|CallReseted))

(event EventBeginPlay
  (bind _defaultsceneroot (Variables|Default|GetDefaultSceneRoot))
  (bind _returnvalue (Transformation|GetWorldLocation _defaultsceneroot))
  (bind (_x _y) (Math|Vector|BreakVector _returnvalue))
  (Variables|Default|SetResetPos _returnvalue)
  (Variables|Default|SetX (Math|Float|Truncate _x))
  (Variables|Default|SetY (Math|Float|Truncate _y)))

(event EventTick
  (params (DeltaSeconds :type Float%20%28single-precision%29))
  (Transformation|SetWorldLocation (Variables|Default|GetDefaultSceneRoot) (Math|Vector|MakeVector (Math|Conversions|ToFloat(Integer) (Variables|Default|GetX)) (Math|Conversions|ToFloat(Integer) (Variables|Default|GetY)) 0.0) false false))

(event Input|AxisEvents|InputAxisMoveForward
  (params (AxisValue :type Float%20%28single-precision%29))
  (if (Variables|Default|GetActive)
    (Utilities|FlowControl|Sequence
      (:then_0
        (if (> AxisValue 0.0)
          (if (< (+ (Variables|Default|GetX) (Variables|Default|GetSquareSize)) (.X (Math|Vector2D|BreakVector2D (Variables|Default|GetMaxLimits))))
            (if (== (Variables|Default|GetXMoved) false)
              (Variables|Default|SetXMoved true)
              (Variables|Default|SetX (+ (Variables|Default|GetX) (Variables|Default|GetSquareSize)))
              (Audio|Components|Audio|Play (Variables|Default|GetBoing) 0.8 :!label _label)))))
      (:then_1
        (if (< AxisValue 0.0)
          (if (> (- (Variables|Default|GetX) (Variables|Default|GetSquareSize)) (.X (Math|Vector2D|BreakVector2D (Variables|Default|GetMinLimits))))
            (if (== (Variables|Default|GetXMoved) false)
              (Variables|Default|SetXMoved true)
              (Variables|Default|SetX (- (Variables|Default|GetX) (Variables|Default|GetSquareSize)))
              (goto _label)))))
      (:then_2
        (if (== AxisValue 0.0)
          (Variables|Default|SetXMoved false))))))

(event Input|AxisEvents|InputAxisMoveRight
  (params (AxisValue :type Float%20%28single-precision%29))
  (if (Variables|Default|GetActive)
    (Utilities|FlowControl|Sequence
      (:then_0
        (if (> AxisValue 0.0)
          (if (< (+ (Variables|Default|GetY) (Variables|Default|GetSquareSize)) (.Y (Math|Vector2D|BreakVector2D (Variables|Default|GetMaxLimits))))
            (if (== (Variables|Default|GetYMoved) false)
              (Variables|Default|SetYMoved true)
              (Variables|Default|SetY (+ (Variables|Default|GetY) (Variables|Default|GetSquareSize)))
              (Audio|Components|Audio|Play (Variables|Default|GetBoing) 0.8 :!label _label)))))
      (:then_1
        (if (< AxisValue 0.0)
          (if (> (- (Variables|Default|GetY) (Variables|Default|GetSquareSize)) (.Y (Math|Vector2D|BreakVector2D (Variables|Default|GetMinLimits))))
            (if (== (Variables|Default|GetYMoved) false)
              (Variables|Default|SetYMoved true)
              (Variables|Default|SetY (- (Variables|Default|GetY) (Variables|Default|GetSquareSize)))
              (goto _label)))))
      (:then_2
        (if (== AxisValue 0.0)
          (Variables|Default|SetYMoved false))))))

(fn ConstructionScript)