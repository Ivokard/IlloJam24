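; BP_CarSpawner is a spawner that endlessly creates random cars from its Cars list at its root location.
; On BeginPlay it enters a delayed loop, timed by each spawned car's NextCarDelay randomized by up to a fifth either way.
; The Inverted flag selects a variant that spawns cars rotated 180 degrees with their Speed negated, for traffic running the opposite direction.
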(event EventBeginPlay
  (bind _cars (Variables|Default|GetCars))
  (bind _outitem (Utilities|Array|Random _cars))
  (if (Variables|Default|GetInverted)
    (bind _returnvalue (Game|SpawnActorfromClass _outitem (Math|Transform|MakeTransform (Transformation|GetWorldLocation (Variables|Default|GetDefaultSceneRoot)) "0.000000,180.000000,0.000000") "Undefined" "MultiplyWithRoot" 0 0 :!label _label))
    (Variables|/Game/IlloJam/Blueprints/BP_Car.BP_Car_C|SetSpeed _returnvalue (* (Variables|/Game/IlloJam/Blueprints/BP_Car.BP_Car_C|GetSpeed _returnvalue) -1.0))
    (Utilities|FlowControl|Delay (+ (Variables|/Game/IlloJam/Blueprints/BP_Car.BP_Car_C|GetNextCarDelay _returnvalue) (Math|Random|RandomFloatinRange (* (/ (Variables|/Game/IlloJam/Blueprints/BP_Car.BP_Car_C|GetNextCarDelay _returnvalue) 5.0) -1.0) (/ (Variables|/Game/IlloJam/Blueprints/BP_Car.BP_Car_C|GetNextCarDelay _returnvalue) 5.0))))
    (goto _label)
    (else
      (bind _returnvalue_2 (Game|SpawnActorfromClass _outitem (Math|Transform|MakeTransform (Transformation|GetWorldLocation (Variables|Default|GetDefaultSceneRoot))) "Undefined" "MultiplyWithRoot" 0 0 :!label _label_2))
      (Utilities|FlowControl|Delay (+ (Variables|/Game/IlloJam/Blueprints/BP_Car.BP_Car_C|GetNextCarDelay _returnvalue_2) (Math|Random|RandomFloatinRange (* (/ (Variables|/Game/IlloJam/Blueprints/BP_Car.BP_Car_C|GetNextCarDelay _returnvalue_2) 5.0) -1.0) (/ (Variables|/Game/IlloJam/Blueprints/BP_Car.BP_Car_C|GetNextCarDelay _returnvalue_2) 5.0))))
      (goto _label_2))))

(fn ConstructionScript)