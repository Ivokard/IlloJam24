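; BP_FakeBaseball is a baseball stand-in that can be thrown repeatedly along a straight line and flags when it can be hit.
; Throw teleports it back to the position cached at BeginPlay and restarts the Trajectory timeline.
; Each update subtracts the timeline value from its current world Y, so movement accumulates per tick.
; Hitable is true while that Y lies between the MinimalDistance X and Y bounds.
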(event Custom|Throw
  (bind _defaultsceneroot (Variables|Default|GetDefaultSceneRoot))
  (bind _defaultsceneroot_2 (Variables|Default|GetDefaultSceneRoot))
  (bind _minimaldistance (Variables|Default|GetMinimalDistance))
  (bind (_x _y) (Math|Vector2D|BreakVector2D _minimaldistance))
  (bind _returnvalue (Transformation|GetWorldLocation _defaultsceneroot))
  (bind _returnvalue_2 (Transformation|GetWorldLocation _defaultsceneroot_2))
  (bind _y_2 (Math|Vector|BreakVector _returnvalue_2))
  (bind (_x_2 _y_3 _z) (Math|Vector|BreakVector _returnvalue))
  (Transformation|SetWorldLocation (Variables|Default|GetDefaultSceneRoot) (Variables|Default|GetOriginalPosition) false true)
  (bind _trajectory (Timeline|Trajectory PlayFromStart)
    (:Update
      (Transformation|SetWorldLocation (Variables|Default|GetDefaultSceneRoot) (Math|Vector|MakeVector _x_2 (- _y_3 _trajectory) _z) false true)
      (bind _output_get (Variables|Default|SetHitable (and (>= _y_2 _x) (<= _y_2 _y)))))))

(event EventBeginPlay
  (Variables|Default|SetOriginalPosition (Transformation|GetWorldLocation (Variables|Default|GetDefaultSceneRoot))))

(fn ConstructionScript)