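; BP_Audio is a sequential player that works through a list of 2D sounds.
; PlayNext plays the current entry of the Audios array, waits for the sound's duration plus that entry's own delay, then advances the index.
; It calls itself until the array is exhausted, then fires the AudioFinished dispatcher.
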(event Custom|PlayNext
  (bind _audios (Variables|Default|GetAudios))
  (bind _audioindex (Variables|Default|GetAudioIndex))
  (bind _output (Utilities|Array|Get(acopy) _audios _audioindex))
  (bind (_sound _delay) (Utilities|Struct|BreakS_AudioData _output))
  (Audio|PlaySound2D _sound 1.0 1.0 0.0 0 0)
  (Utilities|FlowControl|Delay (+ (Variables|/Script/Engine.SoundBase|GetDuration _sound) _delay))
  (bind _result (Math|Integer|IncrementInt (Variables|Default|GetAudioIndex))
    (:%20%20
      (if (<= _result (- (Utilities|Array|Length (Variables|Default|GetAudios)) 1))
        (CallFunction|PlayNext)
        (else
          (Default|CallAudioFinished))))))

(fn ConstructionScript)